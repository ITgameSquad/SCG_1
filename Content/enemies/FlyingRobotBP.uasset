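; Flying robot enemy that nudges itself vertically away from actors entering its Sphere trigger.
; On begin overlap it compares its Z with the sweep result's hit actor and teleport-free, unswept SetActorLocation steps it up if higher, otherwise down, by a small fixed offset.
; End overlap clears IsHit, which nothing in these graphs sets or reads.
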(event OnComponentBeginOverlap(Sphere)
  (params (OtherActor :type Actor%20Object%20Reference) (OtherComp :type Primitive%20Component%20Object%20Reference) (OtherBodyIndex :type Integer) (bFromSweep :type Boolean) (SweepResult :type Hit%20Result%20Structure%20%28by%20ref%29))
  (bind _returnvalue (Transformation|GetActorLocation))
  (bind (_x _y _z) (Math|Vector|BreakVector _returnvalue))
  (if (> _z (.Z (Math|Vector|BreakVector (Transformation|GetActorLocation (.HitActor (Collision|BreakHitResult SweepResult))))))
    (Transformation|SetActorLocation (Math|Vector|MakeVector _x _y (+ _z 1e+01)) false false)
    (else
      (Transformation|SetActorLocation (Math|Vector|MakeVector _x _y (- _z 1e+01)) false false))))

(event OnComponentEndOverlap(Sphere)
  (params (OtherActor :type Actor%20Object%20Reference) (OtherComp :type Primitive%20Component%20Object%20Reference) (OtherBodyIndex :type Integer))
  (Variables|Default|SetIsHit false))

(fn ConstructionScript)