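; Destructible box actor that, once fractured, fades out through its material and then destroys itself.
; On fracture it applies one dynamic material instance to both material slots and starts a looping SetLevelOpacity timer.
; Each tick interpolates InputTime toward zero, using accumulated delta time so the fade accelerates, and spawns an attached decal with that material.
; Once InputTime is near zero, it destroys the actor and clears the timer.
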(event OnComponentFracture(Destructible)
  (params (HitPoint :type Vector%20%28by%20ref%29 :default "0, 0, 0") (HitDirection :type Vector%20%28by%20ref%29 :default "0, 0, 0"))
  (bind _destructible (Variables|Default|GetDestructible))
  (bind _returnvalue (Rendering|Material|CreateDynamicMaterialInstance _destructible 0 (Rendering|Material|GetMaterial _destructible 0) :!class /Script/Engine.PrimitiveComponent))
  (bind _output_get (Variables|Default|SetDynamicMaterialInstance _returnvalue))
  (Rendering|Material|SetMaterial _destructible 0 _output_get)
  (Rendering|Material|SetMaterial _destructible 1 _output_get)
  (bind _returnvalue_2 (Utilities|Time|SetTimerbyFunctionName 0 "SetLevelOpacity" 0.1 true))
  (Variables|Default|SetTimerHandle _returnvalue_2))

(fn ConstructionScript)

(fn SetLevelOpacity
  (bind _dynamicmaterialinstance (Variables|Default|GetDynamicMaterialInstance))
  (bind _output_get (Variables|Default|SetElapsedTime (+ (Utilities|Time|GetWorldDeltaSeconds) (Variables|Default|GetElapsedTime))))
  (bind _returnvalue (Rendering|Material|GetScalarParameterValue _dynamicmaterialinstance "InputTime" :!class /Script/Engine.MaterialInstanceDynamic))
  (if (< _returnvalue 0.01)
    (Actor|DestroyActor)
    (Class|KismetSystemLibrary|ClearTimerHandle (Variables|Default|GetTimerHandle))
    (Variables|Default|SetTimerHandle "")
    (else
      (Rendering|Material|SetScalarParameterValue _dynamicmaterialinstance "InputTime" (Math|Interpolation|FInterpTo _returnvalue 0.0 _output_get 5.0) :!class /Script/Engine.MaterialInstanceDynamic)
      (Class|GameplayStatics|SpawnDecalAttached _dynamicmaterialinstance "0, 0, 0" (Variables|Default|GetDestructible) "None" "0, 0, 0" "0, 0, 0" "KeepWorldPosition" 0.0))))