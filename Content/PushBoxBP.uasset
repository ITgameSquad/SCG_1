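; Pushable box actor that tracks whether it is touching something other than the player character, apparently to block or allow its movement.
; The Box component's begin and end overlap events set and clear a Collusion flag, ignoring the player, with no count of simultaneous overlaps.
; An EnablePhysic function turns on physics simulation for the box; the flag is not read in this Blueprint.
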(event OnComponentEndOverlap(Box)
  (params (OtherActor :type Actor%20Object%20Reference) (OtherComp :type Primitive%20Component%20Object%20Reference) (OtherBodyIndex :type Integer))
  ;[1 1 1] Block/Allow Box Moving
  (if (!= OtherActor (Game|GetPlayerCharacter 0))
    (Variables|Default|SetCollusion false)))

(event OnComponentBeginOverlap(Box)
  (params (OtherActor :type Actor%20Object%20Reference) (OtherComp :type Primitive%20Component%20Object%20Reference) (OtherBodyIndex :type Integer) (bFromSweep :type Boolean) (SweepResult :type Hit%20Result%20Structure%20%28by%20ref%29))
  ;[1 1 1] Block/Allow Box Moving
  (if (!= OtherActor (Game|GetPlayerCharacter 0))
    (Variables|Default|SetCollusion true)))

(event EventBeginPlay)

(event EventActorBeginOverlap
  (params (OtherActor :type Actor%20Object%20Reference)))

(fn ConstructionScript)

(fn EnablePhysic
  (Physics|SetSimulatePhysics (Variables|Default|GetBox) true))